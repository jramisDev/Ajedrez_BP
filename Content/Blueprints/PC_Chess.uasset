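; Player controller for a turn-based chess game, showing the mouse cursor and picking pieces and cells with profile-filtered cursor traces.
; Left click selects a piece of the player whose turn it is and shows its available cells.
; Right click moves it or attacks an enemy cell, then clears cell markings and passes the turn through the cached GM_Game.
; Attacking one specific piece type, likely the king, quits the game instead.
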(event `self.ReceiveBeginPlay`
  (`WidgetBlueprintLibrary.SetInputMode_GameAndUIEx` self null)
  (set `self.bShowMouseCursor` true))

(event `Key|LeftMouseButton`
  (params (Key :type "Key Structure"))
  (bind (_worldlocation _worlddirection) (`self.DeprojectMousePositionToWorld`))
  (:`Pressed`
    (bind _outhit (`KismetSystemLibrary.LineTraceSingleByProfile` _worldlocation (+ _worldlocation (* _worlddirection 5000.0)) "ChessPieceOnly"))
    (if true
      (bind _asbase_chess_piece (cast `/Game/Blueprints/Pieces/BaseChessPiece` (`.HitActor` (`GameplayStatics.BreakHitResult` _outhit))))
      (if (== (`/Game/Blueprints/Pieces/BaseChessPiece.Player1` _asbase_chess_piece) (`/Game/Blueprints/GM_Game.PlayerPlaying` (`self.getGMRef`)))
        (bind _output_get (set `self.SelectedPiece` _asbase_chess_piece))
        (`/Game/Blueprints/Pieces/BaseChessPiece.ShowAvailableCells` _output_get)))))

(event `Key|RightMouseButton`
  (params (Key :type "Key Structure"))
  (bind (_worldlocation _worlddirection) (`self.DeprojectMousePositionToWorld`))
  (bind _as_gm_game (`self.getGMRef`))
  (bind _selectedpiece (`self.SelectedPiece`))
  (:`Pressed`
    (`self.SelectedPiece`
      (:`then`
        (bind (_outhit _returnvalue) (`KismetSystemLibrary.LineTraceSingleByProfile` _worldlocation (+ _worldlocation (* _worlddirection 5000.0)) "OnlyGrid"))
        (if _returnvalue
          (bind _asbp_cell (cast `/Game/Blueprints/BP_Cell` (`.HitActor` (`GameplayStatics.BreakHitResult` _outhit))))
          (if (`/Game/Blueprints/Pieces/BaseChessPiece.Can I Move to Cell` (`self.SelectedPiece`) _asbp_cell)
            (`/Game/Blueprints/BP_Cell.emptyContent` (`BlueprintMapLibrary.Map_Find` (`/Game/Blueprints/GM_Game.Board` (`self.getGMRef`)) (`/Game/Blueprints/Pieces/BaseChessPiece.Coordinate` (`self.SelectedPiece`))))
            (`/Game/Blueprints/Pieces/BaseChessPiece.MoveToCell` (`self.SelectedPiece`) _asbp_cell)
            (`/Game/Blueprints/GM_Game.UnMarkCells` _as_gm_game :!label _label)
            (set `self.SelectedPiece` null)
            (`/Game/Blueprints/GM_Game.NextTurn` _as_gm_game)
            (elif (and (`/Game/Blueprints/BP_Cell.isEnemy` _asbp_cell (`/Game/Blueprints/Pieces/BaseChessPiece.Player1` _selectedpiece)) (`KismetArrayLibrary.Array_Contains` (`/Game/Blueprints/Pieces/BaseChessPiece.WhereCanIAttack` _selectedpiece) (`/Game/Blueprints/BP_Cell.Coordinate` _asbp_cell)))
              (if (`|EnumEquality` (`/Game/Blueprints/Pieces/BaseChessPiece.ChessPiece` (`/Game/Blueprints/BP_Cell.ChessPiece` _asbp_cell)) "NewEnumerator4")
                (`KismetSystemLibrary.QuitGame` null "Quit")
                (else
                  (`/Game/Blueprints/BP_Cell.AttackTo` _asbp_cell (`self.SelectedPiece`))
                  (goto _label)))))))
      (:`else`))))

(fn `getGMRef`
  (returns (`As GM Game` :type "/Game/Blueprints/GM_Game Object Reference"))
  (`self.As GM Game`
    (:`then`
      _)
    (:`else`
      (bind _asgm_game (cast `/Game/Blueprints/GM_Game` (`GameplayStatics.GetGameMode`)))
      (set `self.As GM Game` _asgm_game)))
  (return (`self.As GM Game`)))

(fn `UserConstructionScript`)