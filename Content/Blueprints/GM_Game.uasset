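; Chess game mode that builds the board, spawns both sides' pieces and tracks whose turn it is.
; On BeginPlay it spawns a grid of BP_Cell actors into a coordinate-keyed Board map, places pieces by type, then starts the first turn.
; SpawnPiece destroys any piece its cell rejects.
; Helpers validate coordinates, look up cells and highlight moves or attacks, tracking marked cells for clearing; NextTurn alternates players by turn parity.
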(event `self.ReceiveBeginPlay`
  (bind (_griddimension_x _griddimension_y) (break `/Game/Structs/S_Coordenate` (`self.GridDimension`)))
  (`self.CreateGrid` _griddimension_x _griddimension_y)
  (`self.spawnPieces`)
  (`self.NextTurn`))

(fn `AddSelectedCell`
  (params (NewCell :type "/Game/Blueprints/BP_Cell Object Reference"))
  (`KismetArrayLibrary.Array_AddUnique` (`self.OldSelected`) NewCell))

(fn `Clamp Coordinate`
  (params (Coordinate :type "/Game/Structs/S_Coordenate Structure"))
  (returns (X :type Integer) (Y :type Integer))
  (bind _griddimension_x (break `/Game/Structs/S_Coordenate` (`self.GridDimension`)))
  (bind (_griddimension_x_2 _griddimension_y) (break `/Game/Structs/S_Coordenate` (`self.GridDimension`)))
  (return (`KismetMathLibrary.Clamp` Coordinate_X_5_96A91A7140522DF1CA383F9274AEA856 0 _griddimension_x) (`KismetMathLibrary.Clamp` Coordinate_Y_6_B25D3D454634D02E220555B6FE41D8EE 0 _griddimension_y)))

(fn `CoordinateIsValid`
  (params (Coordinate :type "/Game/Structs/S_Coordenate Structure"))
  (returns (isValid :type Boolean))
  (bind (_griddimension_x _griddimension_y) (break `/Game/Structs/S_Coordenate` (`self.GridDimension`)))
  (return (not (or (> Coordinate_X_5_96A91A7140522DF1CA383F9274AEA856 _griddimension_x) (> Coordinate_Y_6_B25D3D454634D02E220555B6FE41D8EE _griddimension_y) (< Coordinate_X_5_96A91A7140522DF1CA383F9274AEA856 0) (< Coordinate_Y_6_B25D3D454634D02E220555B6FE41D8EE 0)))))

(fn `CreateGrid`
  (params (Width :type Integer) (Height :type Integer))
  (locals (X :type Integer) (Y :type Integer))
  (bind _s_coordenate (make `/Game/Structs/S_Coordenate` (`local.X`) (`local.Y`)))
  (for _index (range (+ Width 1))
    (set `local.X` _index)
    (for _index_2 (range (+ Height 1))
      (set `local.Y` _index_2)
      (bind _returnvalue (`|SpawnActorFromClass` "/Game/Blueprints/BP_Cell.BP_Cell_C" (`KismetMathLibrary.MakeTransform` (`KismetMathLibrary.MakeVector` (`KismetMathLibrary.Conv_IntToDouble` (* (`local.Y`) 100)) (`KismetMathLibrary.Conv_IntToDouble` (* (`local.X`) 100)))) "Undefined" "OverrideRootScale" null _s_coordenate null))
      (`BlueprintMapLibrary.Map_Add` (`self.Board`) _s_coordenate _returnvalue))))

(fn `getCellByCoordinate`
  (params (Coord :type "/Game/Structs/S_Coordenate Structure"))
  (returns (Cell :type "/Game/Blueprints/BP_Cell Object Reference"))
  (return (`BlueprintMapLibrary.Map_Find` (`self.Board`) Coord)))

(fn `MarkCellsForAttacks`
  (params (Coordenate :type "Array of /Game/Structs/S_Coordenate Structure"))
  (for _array_element Coordenate
    (bind _value (`BlueprintMapLibrary.Map_Find` (`self.Board`) _array_element))
    (`/Game/Blueprints/BP_Cell.setStatus` _value "NewEnumerator3")
    (`KismetArrayLibrary.Array_Add` (`self.OldSelected`) _value)))

(fn `MarkCellsForMovement`
  (params (Coordenate :type "Array of /Game/Structs/S_Coordenate Structure"))
  (`self.UnMarkCells`)
  (for _array_element Coordenate
    (bind _value (`BlueprintMapLibrary.Map_Find` (`self.Board`) _array_element))
    (`/Game/Blueprints/BP_Cell.setStatus` _value "NewEnumerator2")
    (`KismetArrayLibrary.Array_Add` (`self.OldSelected`) _value)))

(fn `NextTurn`
  (bind _result (`/Engine/EditorBlueprintResources/StandardMacros.IncrementInt` (`self.Turn`))
    (:`  `
      (bind _output_get (set `self.PlayerPlaying` (== (mod _result 2) 0)))
      (`KismetSystemLibrary.PrintText` (`|FormatText` "Player: {p}" (select `bool` _output_get :`false` "Negras" :`true` "Blancas")) true true (struct :`R` 0.124836 :`G` 1.0 :`A` 1.0) 10.0))))

(fn `SpawnPiece`
  (params (Coordinate :type "/Game/Structs/S_Coordenate Structure (by ref)") (ChessPiece :type "/Game/Enums/E_ChessPiece Enum" :default "NewEnumerator0") (`Player 1` :type Boolean))
  (locals (Base :type "/Game/Blueprints/Pieces/BaseChessPiece Class Reference"))
  (bind _returnvalue (`|SpawnActorFromClass` (select `/Game/Enums/E_ChessPiece` ChessPiece :`NewEnumerator0` "/Game/Blueprints/Pieces/ChessPawn.ChessPawn_C" :`NewEnumerator1` "/Game/Blueprints/Pieces/ChessTower.ChessTower_C" :`NewEnumerator2` "/Game/Blueprints/Pieces/CheesHorse.CheesHorse_C" :`NewEnumerator3` "/Game/Blueprints/Pieces/ChessBishop.ChessBishop_C" :`NewEnumerator4` "/Game/Blueprints/Pieces/ChessKing.ChessKing_C" :`NewEnumerator5` "/Game/Blueprints/Pieces/ChessQueen.ChessQueen_C" :!type "/Game/Blueprints/Pieces/BaseChessPiece Class Reference") (`KismetMathLibrary.MakeTransform` (0.0 0.0 0.0)) "AlwaysSpawn" "OverrideRootScale" null Coordinate `Player 1` null))
  (bind _cansetcontent (`/Game/Blueprints/BP_Cell.setContent` (`BlueprintMapLibrary.Map_Find` (`self.Board`) Coordinate) _returnvalue))
  (if (not _cansetcontent)
    (`KismetSystemLibrary.PrintString` "Casilla ya ocupada" true true (struct :`R` 1.0 :`A` 1.0))
    (`self.K2_DestroyActor` _returnvalue)))

(fn `spawnPieces`
  (locals (Player1 :type Boolean))
  (bind (_griddimension_x _griddimension_y) (break `/Game/Structs/S_Coordenate` (`self.GridDimension`)))
  (bind _griddimension_x_2 (break `/Game/Structs/S_Coordenate` (`self.GridDimension`)))
  (bind _griddimension_x_3 (break `/Game/Structs/S_Coordenate` (`self.GridDimension`)))
  (bind _griddimension_x_4 (break `/Game/Structs/S_Coordenate` (`self.GridDimension`)))
  (bind (_griddimension_x_5 _griddimension_y_2) (break `/Game/Structs/S_Coordenate` (`self.GridDimension`)))
  (bind _griddimension_x_6 (break `/Game/Structs/S_Coordenate` (`self.GridDimension`)))
  (for _index (range 2)
    (set `local.Player1` (== _index 1))
    ;[1 1 1] Spawn Peones
    (for _index_2 (range (+ _griddimension_x_2 1))
      (`self.SpawnPiece` (make `/Game/Structs/S_Coordenate` _index_2 (select `int` _index :`0` 6 :`1` 1)) "NewEnumerator0" (`local.Player1`)))
    ;[1 1 1] Spawn Torres
    (for _index_3 (range 2)
      (`self.SpawnPiece` (make `/Game/Structs/S_Coordenate` (select `int` _index_3 :`0` 0 :`1` _griddimension_x_3) (select `bool` (`local.Player1`) :`false` _griddimension_x_3)) "NewEnumerator1" (`local.Player1`)))
    ;[1 1 1] Spawn Caballos
    (for _index_4 (range 2)
      (`self.SpawnPiece` (make `/Game/Structs/S_Coordenate` (select `int` _index_4 :`0` 1 :`1` (- _griddimension_x_6 1)) (select `bool` (`local.Player1`) :`false` _griddimension_x_6)) "NewEnumerator2" (`local.Player1`)))
    ;[1 1 1] Spawn Bishop
    (for _index_5 (range 2)
      (`self.SpawnPiece` (make `/Game/Structs/S_Coordenate` (select `int` _index_5 :`0` 2 :`1` (- _griddimension_x_4 2)) (select `bool` (`local.Player1`) :`false` _griddimension_x_4)) "NewEnumerator3" (`local.Player1`)))
    ;[1 1 1] Spawn Queen
    (for _ (range 2)
      (`self.SpawnPiece` (make `/Game/Structs/S_Coordenate` 3 (select `bool` (`local.Player1`) :`false` _griddimension_y_2)) "NewEnumerator5" (`local.Player1`)))
    ;[1 1 1] Spawn King
    (for _ (range 2)
      (`self.SpawnPiece` (make `/Game/Structs/S_Coordenate` 4 (select `bool` (`local.Player1`) :`false` _griddimension_y)) "NewEnumerator4" (`local.Player1`)))))

(fn `UnMarkCells`
  (for _array_element (`self.OldSelected`)
    (`/Game/Blueprints/BP_Cell.setStatus` _array_element "NewEnumerator0"))
  (`KismetArrayLibrary.Array_Clear` (`self.OldSelected`)))

(fn `UserConstructionScript`)