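; BP_Cell is one chess board square that shows its coordinate and tracks the piece on it.
; It attaches and releases pieces, answers occupancy and enemy queries, and resolves captures by destroying the occupant, clearing the attacker's old cell through GM_Game and taking the attacker.
; A dynamic material draws the checker shade from coordinate parity and tints the square by status through a color map.
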(event `self.ReceiveBeginPlay`
  (bind (_coordinate_x _coordinate_y) (break `/Game/Structs/S_Coordenate` (`self.Coordinate`)))
  (`TextRenderComponent.K2_SetText` (`self.TextRender`) (`|FormatText` "({X},{Y})" _coordinate_x _coordinate_y))
  (`self.setMaterialColor`))

(fn `AttackTo`
  (params (Attacker :type "/Game/Blueprints/Pieces/BaseChessPiece Object Reference"))
  (bind _chesspiece (`self.ChessPiece`)
    (:`then`
      (`self.K2_DestroyActor` _chesspiece)
      (`self.emptyContent`)
      (`self.emptyContent` (`/Game/Blueprints/GM_Game.getCellByCoordinate` (`self.getGMRef`) (`/Game/Blueprints/Pieces/BaseChessPiece.Coordinate` Attacker)))
      (`self.setContent` Attacker))
    (:`else`)))

(fn `emptyContent`
  (set `self.ChessPiece` null)
  (set `self.Status` "NewEnumerator0")
  (`self.setMaterialColor`))

(fn `getGMRef`
  (returns (`As GM Game` :type "/Game/Blueprints/GM_Game Object Reference"))
  (`self.GameMode`
    (:`then`
      _)
    (:`else`
      (bind _asgm_game (cast `/Game/Blueprints/GM_Game` (`GameplayStatics.GetGameMode`)))
      (set `self.GameMode` _asgm_game)))
  (return (`self.GameMode`)))

(fn `isEnemy`
  (params (YourTeam :type Boolean))
  (returns (ReturnValue :type Boolean))
  (if (`self.isFull`)
    (return (!= (`/Game/Blueprints/Pieces/BaseChessPiece.Player1` (`self.ChessPiece`)) YourTeam))
    (else
      (return false))))

(fn `isFull`
  (returns (`Is Full` :type Boolean))
  (return (`KismetSystemLibrary.IsValid` (`self.ChessPiece`))))

(fn `setContent`
  (params (ChessPiece :type "/Game/Blueprints/Pieces/BaseChessPiece Object Reference"))
  (returns (CanSetContent :type Boolean))
  (`self.ChessPiece`
    (:`then`
      (return false))
    (:`else`
      (bind _output_get (set `self.ChessPiece` ChessPiece))
      (`self.K2_AttachToComponent` _output_get (`self.Scene`) "None" "SnapToTarget" "KeepWorld" "KeepWorld" true)
      (set `/Game/Blueprints/Pieces/BaseChessPiece.Coordinate` (`self.Coordinate`) (`self.ChessPiece`))
      (`self.setStatus` "NewEnumerator1")
      (`self.setMaterialColor`)
      (return true))))

(fn `setMaterialColor`
  (bind (_coordinate_x _coordinate_y) (break `/Game/Structs/S_Coordenate` (`self.Coordinate`)))
  (`self.MaterialInstance`
    (:`then`
      _)
    (:`else`
      (bind _returnvalue (`PrimitiveComponent.CreateDynamicMaterialInstance` (`self.Cube`) 0 "/Game/Material/M_Cell.M_Cell" "None"))
      (set `self.MaterialInstance` _returnvalue)
      (`MaterialInstanceDynamic.SetScalarParameterValue` (`self.MaterialInstance`) "White" (select `bool` (== (mod (+ _coordinate_x _coordinate_y) 2) 0) :`true` 1.0 :!type "Float (single-precision)"))))
  (`MaterialInstanceDynamic.SetVectorParameterValue` (`self.MaterialInstance`) "BaseColor" (`BlueprintMapLibrary.Map_Find` (`self.ColorCell`) (`self.Status`))))

(fn `setStatus`
  (params (Status :type "/Game/Enums/E_CellStatus Enum" :default "NewEnumerator0"))
  (if (`|EnumEquality` Status "NewEnumerator0")
    (set `self.Status` (select `bool` (`self.isFull`) :`false` "NewEnumerator0" :`true` "NewEnumerator1" :!type "/Game/Enums/E_CellStatus Enum"))
    (else
      (set `self.Status` Status)))
  (`self.setMaterialColor`))

(fn `UserConstructionScript`)