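; Camera pawn that centers itself over the game grid when play begins.
; On BeginPlay it teleports to an X and Y position scaled from the game mode's GridDimension.
; A helper fetches GM_Game from the current game mode and caches the cast reference for reuse.
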(event `self.ReceiveBeginPlay`
  (bind (_griddimension_x _griddimension_y) (break `/Game/Structs/S_Coordenate` (`/Game/Blueprints/GM_Game.GridDimension` (`self.getGMRef`))))
  (`self.K2_SetActorLocation` (`KismetMathLibrary.MakeVector` (`KismetMathLibrary.Conv_IntToDouble` (* _griddimension_x 50)) (`KismetMathLibrary.Conv_IntToDouble` (* _griddimension_y 50))) false true))

(fn `getGMRef`
  (returns (`As GM Game` :type "/Game/Blueprints/GM_Game Object Reference"))
  (`self.As GM Game`
    (:`then`
      _)
    (:`else`
      (bind _asgm_game (cast `/Game/Blueprints/GM_Game` (`GameplayStatics.GetGameMode`)))
      (set `self.As GM Game` _asgm_game)))
  (return (`self.As GM Game`)))

(fn `UserConstructionScript`)