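; Base chess piece Blueprint that handles team material, move and attack calculation, cell highlighting and moves onto empty cells.
; WhereCanIMove steps along each Increment direction, up to a step limit or unlimited when zero, stopping at board edges and occupied cells.
; That scan also caches enemy coordinates, which WhereCanIAttack returns without recalculating.
; GM_Game supplies board queries and cell marking through a cached reference; TeamFactor gives a per-team sign.
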(event `self.ReceiveBeginPlay`
  (for _array_element (`SceneComponent.GetChildrenComponents` (`self.GraphicsHere`) true)
    (bind _asstatic_mesh_component (cast `StaticMeshComponent` _array_element))
    (`PrimitiveComponent.SetMaterial` _asstatic_mesh_component 0 (select `bool` (`self.Player1`) :`false` "/Game/Material/M_CheessPieceBlack.M_CheessPieceBlack" :`true` "/Game/Material/M_CheessPieceWhite.M_CheessPieceWhite" :!type "MaterialInterface Object Reference"))))

(fn `Can I Move to Cell`
  (params (Cell :type "/Game/Blueprints/BP_Cell Object Reference"))
  (returns (`Yes We Can` :type Boolean))
  (if (`/Game/Blueprints/BP_Cell.isFull` Cell)
    (return false)
    (else
      (return (>= (`KismetArrayLibrary.Array_Find` (`self.WhereCanIMove`) (`/Game/Blueprints/BP_Cell.Coordinate` (`local.Cell`))) 0)))))

(fn `getGMRef`
  (returns (`As GM Game` :type "/Game/Blueprints/GM_Game Object Reference"))
  (`self.As GM Game`
    (:`then`
      _)
    (:`else`
      (bind _asgm_game (cast `/Game/Blueprints/GM_Game` (`GameplayStatics.GetGameMode`)))
      (set `self.As GM Game` _asgm_game)))
  (return (`self.As GM Game`)))

(fn `MoveToCell`
  (params (Cell :type "/Game/Blueprints/BP_Cell Object Reference"))
  (returns (CanSetContent :type Boolean))
  (if (`self.Can I Move to Cell` Cell)
    (bind _cansetcontent (`/Game/Blueprints/BP_Cell.setContent` Cell self))
    (set `self.Coordinate` (`/Game/Blueprints/BP_Cell.Coordinate` (`local.Cell`)))
    (return _cansetcontent)
    (else
      (return false))))

(fn `ShowAvailableCells`
  (`/Game/Blueprints/GM_Game.UnMarkCells` (`self.getGMRef`))
  (`/Game/Blueprints/GM_Game.MarkCellsForMovement` (`self.getGMRef`) (`self.WhereCanIMove`))
  (`/Game/Blueprints/GM_Game.MarkCellsForAttacks` (`self.getGMRef`) (`self.WhereCanIAttack`)))

(fn `TeamFactor`
  (returns (Factor :type Integer))
  (if (`self.Player1`)
    (return 1)
    (else
      (return -1))))

(fn `UserConstructionScript`)

(fn `WhereCanIAttack`
  (returns (Coordinates :type "Array of /Game/Structs/S_Coordenate Structure"))
  (return (`self.CoordinateToKill`)))

(fn `WhereCanIMove`
  (returns (CoordinatesAvaible :type "Array of /Game/Structs/S_Coordenate Structure"))
  (locals (InitialCoordinate :type "/Game/Structs/S_Coordenate Structure") (CellAvaible :type Boolean) (NewCoordinate :type "/Game/Structs/S_Coordenate Structure") (CoordinateToReturn :type "Array of /Game/Structs/S_Coordenate Structure") (Incremented :type Integer))
  (bind _as_gm_game (`self.getGMRef`))
  (bind _newcoordinate (`local.NewCoordinate`))
  (bind _numberoftimestodoincrement (`self.NumberOfTimesToDoIncrement`))
  (bind _cell (`/Game/Blueprints/GM_Game.getCellByCoordinate` _as_gm_game _newcoordinate))
  (`KismetArrayLibrary.Array_Clear` (`self.CoordinateToKill`))
  (for _array_element (`self.Increment`)
    (set `local.InitialCoordinate` (`self.Coordinate`))
    (set `local.Incremented` 0)
    (set `local.CellAvaible` true)
    (while (`local.CellAvaible`)
      (if (or (> _numberoftimestodoincrement (`local.Incremented`)) (== _numberoftimestodoincrement 0))
        (`/Engine/EditorBlueprintResources/StandardMacros.IncrementInt` (`local.Incremented`)
          (:`  `
            (set `local.NewCoordinate` (`/Game/Library/BPL_SoyVago.SumCoordinate` (`local.InitialCoordinate`) _array_element))
            (if (`/Game/Blueprints/GM_Game.CoordinateIsValid` _as_gm_game _newcoordinate)
              (if (`/Game/Blueprints/BP_Cell.isFull` _cell)
                (if (`/Game/Blueprints/BP_Cell.isEnemy` _cell (`self.Player1`))
                  (`KismetArrayLibrary.Array_AddUnique` (`self.CoordinateToKill`) (`local.NewCoordinate`))
                  (set `local.CellAvaible` false)
                  (else
                    (set `local.CellAvaible` false)))
                (else
                  (`KismetArrayLibrary.Array_AddUnique` (`local.CoordinateToReturn`) (`local.NewCoordinate`))
                  (set `local.InitialCoordinate` (`local.NewCoordinate`))))
              (else
                (set `local.CellAvaible` false)))))
        (else
          (set `local.CellAvaible` false)))))
  (return (`local.CoordinateToReturn`)))