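; Chess rook (tower) piece that works out which grid cells it can move to and attack.
; WhereCanIMove uses nested axis and direction loops to scan four straight lines through the game manager's grid, collecting empty cells until the first occupied one.
; Those blocking cells become kill candidates, which WhereCanIAttack filters to enemies, so it relies on the move scan having run.
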(fn `UserConstructionScript`
  (`parent.UserConstructionScript`))

(fn `WhereCanIAttack`
  (returns (Coordinates :type "Array of /Game/Structs/S_Coordenate Structure"))
  (locals (TrueCoordinatesToKill :type "Array of /Game/Structs/S_Coordenate Structure"))
  (for _array_element (`self.CoordinatesToKill`)
    (if (`/Game/Blueprints/BP_Cell.isEnemy` (`/Game/Blueprints/GM_Game.getCellByCoordinate` (`self.getGMRef`) _array_element) (`self.Player1`))
      (`KismetArrayLibrary.Array_AddUnique` (`local.TrueCoordinatesToKill`) _array_element)))
  (return (`local.TrueCoordinatesToKill`)))

(fn `WhereCanIMove`
  (returns (CoordinatesAvaible :type "Array of /Game/Structs/S_Coordenate Structure"))
  (locals (Coordinates :type "Array of /Game/Structs/S_Coordenate Structure") (isInY :type Boolean) (Suma :type Boolean) (UseX :type Boolean))
  (bind (_coordinate_x _coordinate_y) (break `/Game/Structs/S_Coordenate` (`self.Coordinate`)))
  (bind (_coordinate_x_2 _coordinate_y_2) (break `/Game/Structs/S_Coordenate` (`self.Coordinate`)))
  (bind _coordinate_x_3 (break `/Game/Structs/S_Coordenate` (`self.Coordinate`)))
  (bind (_coordinate_x_4 _coordinate_y_3) (break `/Game/Structs/S_Coordenate` (`self.Coordinate`)))
  (bind _returnvalue (select `bool` (`local.UseX`) :`false` _coordinate_y_2 :`true` _coordinate_x_2))
  (bind (_griddimension_x _griddimension_y) (break `/Game/Structs/S_Coordenate` (`/Game/Blueprints/GM_Game.GridDimension` (`self.getGMRef`))))
  (`KismetArrayLibrary.Array_Clear` (`self.CoordinatesToKill`))
  (for _index (range 2)
    (set `local.UseX` (== _index 0))
    (for _index_2 (range 2)
      (set `local.Suma` (== _index_2 0))
      (for _index_3 (range 1 (+ (select `bool` (`local.Suma`) :`false` _returnvalue :`true` (- (select `bool` (`local.UseX`) :`false` _griddimension_y :`true` _griddimension_x) _returnvalue)) 1))
        (bind _returnvalue_2 (+ (select `bool` (`local.UseX`) :`false` _coordinate_y :`true` _coordinate_x) (* _index_3 (select `bool` (`local.Suma`) :`false` -1 :`true` 1))))
        (bind _s_coordenate (make `/Game/Structs/S_Coordenate` (select `bool` (`local.UseX`) :`false` _coordinate_x_3 :`true` _returnvalue_2) (select `bool` (`local.UseX`) :`false` _returnvalue_2 :`true` _coordinate_y_3)))
        (if (`/Game/Blueprints/BP_Cell.isFull` (`/Game/Blueprints/GM_Game.getCellByCoordinate` (`self.getGMRef`) _s_coordenate))
          (`KismetArrayLibrary.Array_AddUnique` (`self.CoordinatesToKill`) _s_coordenate)
          (break)
          (else
            (`KismetArrayLibrary.Array_AddUnique` (`local.Coordinates`) _s_coordenate))))))
  (return (`local.Coordinates`)))