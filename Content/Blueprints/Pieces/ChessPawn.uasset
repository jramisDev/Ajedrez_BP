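; ChessPawn is a chess piece Blueprint that computes a pawn's legal destination and capture cells on the board.
; WhereCanIMove adds the empty cell ahead, plus the cell two ahead from the starting row, checked independently of the first.
; WhereCanIAttack adds valid forward cells at the column offsets in Valores that hold an enemy.
; Both query cells through the GM reference and use TeamFactor to set direction per player.
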(fn `UserConstructionScript`
  (`parent.UserConstructionScript`))

(fn `WhereCanIAttack`
  (returns (Coordinates :type "Array of /Game/Structs/S_Coordenate Structure"))
  (locals (TMPArray :type "Array of /Game/Structs/S_Coordenate Structure") (Valores :type "Array of Integer"))
  (bind _as_gm_game (`self.getGMRef`))
  (bind (_coordinate_x _coordinate_y) (break `/Game/Structs/S_Coordenate` (`self.Coordinate`)))
  (for _array_element (`local.Valores`)
    (bind _s_coordenate (make `/Game/Structs/S_Coordenate` (+ _coordinate_x _array_element) (+ _coordinate_y (`self.TeamFactor`))))
    (if (`/Game/Blueprints/GM_Game.CoordinateIsValid` _as_gm_game _s_coordenate)
      (if (`/Game/Blueprints/BP_Cell.isEnemy` (`/Game/Blueprints/GM_Game.getCellByCoordinate` _as_gm_game _s_coordenate) (`self.Player1`))
        (`KismetArrayLibrary.Array_AddUnique` (`local.TMPArray`) _s_coordenate))))
  (return (`local.TMPArray`)))

(fn `WhereCanIMove`
  (returns (CoordinatesAvaible :type "Array of /Game/Structs/S_Coordenate Structure"))
  (locals (TMPArray :type "Array of /Game/Structs/S_Coordenate Structure"))
  (bind (_coordinate_x _coordinate_y) (break `/Game/Structs/S_Coordenate` (`self.Coordinate`)))
  (bind (_coordinate_x_2 _coordinate_y_2) (break `/Game/Structs/S_Coordenate` (`self.Coordinate`)))
  (bind _s_coordenate (make `/Game/Structs/S_Coordenate` _coordinate_x_2 (+ _coordinate_y_2 (`self.TeamFactor`))))
  (bind _s_coordenate_2 (make `/Game/Structs/S_Coordenate` _coordinate_x (+ _coordinate_y (* (`self.TeamFactor`) 2))))
  ;[1 1 1] (X,Y+1)
  (if (not (`/Game/Blueprints/BP_Cell.isFull` (`/Game/Blueprints/GM_Game.getCellByCoordinate` (`self.getGMRef`) _s_coordenate)))
    (`KismetArrayLibrary.Array_AddUnique` (`local.TMPArray`) _s_coordenate))
  ;[1 1 1] (X,Y+1)
  (if (== _coordinate_y (select `bool` (`self.Player1`) :`false` 6 :`true` 1))
    (if (not (`/Game/Blueprints/BP_Cell.isFull` (`/Game/Blueprints/GM_Game.getCellByCoordinate` (`self.getGMRef`) _s_coordenate_2)))
      (`KismetArrayLibrary.Array_AddUnique` (`local.TMPArray`) _s_coordenate_2)))
  (return (`local.TMPArray`)))