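; Chess knight piece Blueprint that reports the cells it can move to or attack.
; WhereCanIMove builds all eight L-shaped offsets from Coordinate with three nested two-way loops and looks each cell up through the game mode reference.
; Empty cells are returned as moves, while enemy-occupied cells are stored in AttackCoord.
; WhereCanIAttack only returns that stored list, so its result depends on the last move query.
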(fn `UserConstructionScript`
  (`parent.UserConstructionScript`))

(fn `WhereCanIAttack`
  (returns (Coordinates :type "Array of /Game/Structs/S_Coordenate Structure"))
  (return (`self.AttackCoord`)))

(fn `WhereCanIMove`
  (returns (CoordinatesAvaible :type "Array of /Game/Structs/S_Coordenate Structure"))
  (locals (TMPCoord :type "Array of /Game/Structs/S_Coordenate Structure") (Suma :type Boolean) (Arriba :type Boolean) (UseX :type Boolean))
  (bind _as_gm_game (`self.getGMRef`))
  (bind (_coordinate_x _coordinate_y) (break `/Game/Structs/S_Coordenate` (`self.Coordinate`)))
  (bind _returnvalue (select `bool` (`local.Suma`) :`false` -1 :`true` 1))
  (bind _returnvalue_2 (select `bool` (`local.Arriba`) :`false` -2 :`true` 2))
  (bind _s_coordenate (make `/Game/Structs/S_Coordenate` (+ _coordinate_x (select `bool` (`local.UseX`) :`false` _returnvalue_2 :`true` _returnvalue)) (+ _coordinate_y (select `bool` (`local.UseX`) :`false` _returnvalue :`true` _returnvalue_2))))
  (bind _cell (`/Game/Blueprints/GM_Game.getCellByCoordinate` _as_gm_game _s_coordenate))
  (`KismetArrayLibrary.Array_Clear` (`self.AttackCoord`))
  (for _index (range 2)
    (set `local.UseX` (== _index 0))
    (for _index_2 (range 2)
      (set `local.Arriba` (== _index_2 0))
      (for _index_3 (range 2)
        (set `local.Suma` (== _index_3 0))
        (if (`KismetSystemLibrary.IsValid` _as_gm_game)
          (if (`/Game/Blueprints/BP_Cell.isFull` _cell)
            (if (`/Game/Blueprints/BP_Cell.isEnemy` _cell (`self.Player1`))
              (`KismetArrayLibrary.Array_AddUnique` (`self.AttackCoord`) _s_coordenate))
            (else
              (`KismetArrayLibrary.Array_AddUnique` (`local.TMPCoord`) _s_coordenate)))))))
  (return (`local.TMPCoord`)))